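; Hostile actor "bad" that damages the player on contact.
; On capsule overlap with BP_Player it subtracts a fixed, clamped amount of HP once, then either flags death and shows the restart screen or plays a UI animation, and destroys itself.
; Overlap with a NewBlueprint1 actor destroys both actors.
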(event `self.Capsule.OnComponentBeginOverlap`
  (params (OverlappedComponent :type "PrimitiveComponent Object Reference") (OtherActor :type "Actor Object Reference") (OtherComp :type "PrimitiveComponent Object Reference") (OtherBodyIndex :type Integer) (bFromSweep :type Boolean) (SweepResult :type "HitResult Structure (by ref)"))
  (`|ExecutionSequence`
    (:`then_0`
      (bind _asbp_player (cast `/Game/InfiniteMatrix/Blueprints/BP_Player` OtherActor))
      (`/Engine/EditorBlueprintResources/StandardMacros.DoOnce` false
        (:`Completed`
          (bind _output_get (set `/Game/InfiniteMatrix/Blueprints/BP_Player.HP` (`KismetMathLibrary.Clamp` (- (`/Game/InfiniteMatrix/Blueprints/BP_Player.HP` _asbp_player) 10) 0 100) _asbp_player))
          (if (<= _output_get 0)
            (set `/Game/InfiniteMatrix/Blueprints/BP_Player.IsDead` true _asbp_player)
            (`/Game/InfiniteMatrix/Blueprints/BP_Player.DisplayRestart` _asbp_player)
            (else
              (bind _ui (`/Game/InfiniteMatrix/Blueprints/BP_Player.UI` _asbp_player))
              (`UserWidget.PlayAnimation` _ui (`/Game/InfiniteMatrix/UI/HP.1` _ui) 0.0 1 "Forward" 1.0 false)))
          (`self.K2_DestroyActor`))))
    (:`then_1`
      (bind _asnew_blueprint_1 (cast `/Game/InfiniteMatrix/Blueprints/NewBlueprint1` OtherActor))
      (`self.K2_DestroyActor` _asnew_blueprint_1)
      (`self.K2_DestroyActor`))))

(fn `UserConstructionScript`)